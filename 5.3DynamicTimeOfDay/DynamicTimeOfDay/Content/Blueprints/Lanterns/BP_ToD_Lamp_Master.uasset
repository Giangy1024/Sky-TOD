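; Master lamp Blueprint that switches its lights and emissive mesh material on or off, optionally following BP_TimeOfDay's day/night cycle.
; Construction script builds the dynamic material, applies shared color and light settings to all LightComponents, caches the time-of-day actor and previews the ON state.
; BeginPlay briefly waits, binds to set-day/set-night events and sets the initial state from the current hour.
; TurnOn and TurnOff add random delays to stagger switching between lamps.
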(event `self.ReceiveBeginPlay`
  (`KismetSystemLibrary.Delay` 0.04)
  (`self.BindEvents`)
  (`self.StartupOnOff`))

(event `StartupOnOff`
  (bind _output (`|ConvertAsset` (`self.TimeOfDayActor`)))
  (bind (_daystarthour _nightstarthour) (break `DayNightEvents` (`TimeOfDay.DayNightEvents` _output)))
  ;[1 1 1] Startup On Off
  (if (`self.UseWithTimeOfDay`)
    (`/Engine/EditorBlueprintResources/StandardMacros.IsValid` _output
      (:`Is Valid`
        (if (`KismetMathLibrary.InRange_FloatFloat` (`.Hour` (break `BaseSetup` (`TimeOfDay.BaseSetup` _output))) _daystarthour _nightstarthour)
          (`self.SetOFF`)
          (else
            (`self.SetOn`)))))))

(event `BindEvents`
  (bind _output (`|ConvertAsset` (`self.TimeOfDayActor`)))
  ;[1 1 1] Bind Events
  (if (`self.UseWithTimeOfDay`)
    (`/Engine/EditorBlueprintResources/StandardMacros.IsValid` _output
      (:`Is Valid`
        (add `/DynamicTimeOfDay/Blueprints/TimeOfDay/BP_TimeOfDay.SetDay` _output (`|CreateDelegate` :!event `TurnOn`))
        (add `/DynamicTimeOfDay/Blueprints/TimeOfDay/BP_TimeOfDay.SetNight` _output (`|CreateDelegate` :!event `TurnOff`))))))

(event `SetOn`
  (bind _dynmat (`self.DynMat`))
  (`/Engine/EditorBlueprintResources/StandardMacros.IsValid` _dynmat
    (:`Is Valid`
      (`MaterialInstanceDynamic.SetScalarParameterValue` _dynmat "EmissiveScale" (`self.EmissiveScale`)))
    (:`Is Not Valid`
      _))
  (for _array_element (`self.Lights`)
    (`/Engine/EditorBlueprintResources/StandardMacros.IsValid` _array_element
      (:`Is Valid`
        (`SceneComponent.SetVisibility` _array_element true false)))))

(event `SetOFF`
  (bind _dynmat (`self.DynMat`))
  (`/Engine/EditorBlueprintResources/StandardMacros.IsValid` _dynmat
    (:`Is Valid`
      (`MaterialInstanceDynamic.SetScalarParameterValue` _dynmat "EmissiveScale" 0.0))
    (:`Is Not Valid`
      _))
  (for _array_element (`self.Lights`)
    (`/Engine/EditorBlueprintResources/StandardMacros.IsValid` _array_element
      (:`Is Valid`
        (`SceneComponent.SetVisibility` _array_element false false)))))

(event `TurnOn`
  (`KismetSystemLibrary.Delay` (`KismetMathLibrary.RandomFloatInRange` 0.0 1.5))
  (`self.SetOn`))

(event `TurnOff`
  (`KismetSystemLibrary.Delay` (`KismetMathLibrary.RandomFloatInRange` 0.0 1.5))
  (`self.SetOFF`))

(fn `UserConstructionScript`
  (bind _lampmesh (`self.LampMesh`))
  (bind _emissiveid (`self.EmissiveID`))
  (bind _dynmat (`self.DynMat`))
  (bind _color (`self.Color`))
  ;[1 1 1] Dynamic Material Setup
  (`/Engine/EditorBlueprintResources/StandardMacros.IsValid` _lampmesh
    (:`Is Valid`
      (bind _returnvalue (`PrimitiveComponent.CreateDynamicMaterialInstance` _lampmesh _emissiveid (`PrimitiveComponent.GetMaterial` _lampmesh _emissiveid) "None"))
      (set `self.DynMat` _returnvalue)
      ;[1 1 1] Material Setup
      (`MaterialInstanceDynamic.SetScalarParameterValue` _dynmat "EmissiveScale" (`self.EmissiveScale`))
      (`MaterialInstanceDynamic.SetVectorParameterValue` _dynmat "Emissive" _color)
      (`MaterialInstanceDynamic.SetVectorParameterValue` _dynmat "Color" _color)
      ;[1 1 1] Light Setup
      (bind _output_get (set `self.Lights` (`self.K2_GetComponentsByClass` "/Script/Engine.LightComponent")))
      (for _array_element _output_get
        (`/Engine/EditorBlueprintResources/StandardMacros.IsValid` _array_element
          (:`Is Valid`
            (bind _aslight_component (cast `LightComponent` _array_element)
              (:`then`
                (`LightComponent.SetVolumetricScatteringIntensity` _aslight_component (`self.VolumetricScatteringIntensity`))
                (`LightComponent.SetIntensity` _aslight_component (`self.LightIntensity`))
                (`LightComponent.SetLightColor` _aslight_component (`self.Color`) true)
                (`LightComponentBase.SetCastShadows` _aslight_component (`self.CastShadows`))
                (`LightComponentBase.SetCastVolumetricShadow` _aslight_component (`self.CastVolumetricShadows`))
                (`LightComponent.SetIndirectLightingIntensity` _aslight_component (`self.IndirectLightingIntensity`)))
              (:`CastFailed`
                _))
            (bind _aslocal_light_component (cast `LocalLightComponent` _array_element)
              (:`then`
                (`LocalLightComponent.SetAttenuationRadius` _aslocal_light_component (`self.LightRadius`)))
              (:`CastFailed`
                _))
            ;[1 1 1] TimeOfDay Actor Grab
            (if (`self.UseWithTimeOfDay`)
              (bind _returnvalue_2 (`GameplayStatics.GetActorOfClass` "/DynamicTimeOfDay/Blueprints/TimeOfDay/BP_TimeOfDay.BP_TimeOfDay_C"))
              (`/Engine/EditorBlueprintResources/StandardMacros.IsValid` _returnvalue_2
                (:`Is Valid`
                  (set `self.TimeOfDayActor` (`|ConvertAsset` _returnvalue_2)))
                (:`Is Not Valid`
                  _)))
            ;[1 1 1] Set On/Off
            (if (`self.ON?`)
              (`self.SetOn`)
              (else
                (`self.SetOFF`)))))))
    (:`Is Not Valid`)))