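; Firefly VFX actor with a Niagara particle effect and an optional point light, named for time-of-day use.
; SetON and SetOFF events activate or deactivate the particles and show or hide the light.
; The construction script applies the exposed light settings, or destroys the light component when UseLight is off.
; The UseWithTimeOfDay branch is empty, and nothing in these graphs calls the toggle events.
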(event `self.SetON`
  (bind _pointlight (`self.PointLight`))
  (`/Engine/EditorBlueprintResources/StandardMacros.IsValid` (`self.NiagaraSystem`)
    (:`Is Valid`
      (`ActorComponent.Activate` (`self.NiagaraParticle`) true))
    (:`Is Not Valid`
      _))
  (`/Engine/EditorBlueprintResources/StandardMacros.IsValid` _pointlight
    (:`Is Valid`
      (`SceneComponent.SetVisibility` _pointlight true false))))

(event `self.SetOFF`
  (bind _pointlight (`self.PointLight`))
  (`/Engine/EditorBlueprintResources/StandardMacros.IsValid` (`self.NiagaraSystem`)
    (:`Is Valid`
      (`ActorComponent.Deactivate` (`self.NiagaraParticle`)))
    (:`Is Not Valid`
      _))
  (`/Engine/EditorBlueprintResources/StandardMacros.IsValid` _pointlight
    (:`Is Valid`
      (`SceneComponent.SetVisibility` _pointlight false false))))

(fn `UserConstructionScript`
  (bind _pointlight (`self.PointLight`))
  (`parent.UserConstructionScript`)
  (`|ExecutionSequence`
    (:`then_0`
      (if (`self.UseLight?`)
        (`LightComponent.SetLightColor` _pointlight (`self.Color`) true)
        (`LocalLightComponent.SetAttenuationRadius` _pointlight (`self.Radius`))
        (`LightComponentBase.SetCastShadows` _pointlight (`self.CastShadows?`))
        (`LightComponent.SetIntensity` _pointlight (`self.Intensity`))
        (`LightComponent.SetVolumetricScatteringIntensity` _pointlight (`self.VolumetricScattering`))
        (`LightComponent.SetIndirectLightingIntensity` _pointlight (`self.IndirectIntensity`))
        (else
          (`ActorComponent.K2_DestroyComponent` (`self.PointLight`)))))
    (:`then_1`
      (if (`self.UseWithTimeOfDay`)
        _))))