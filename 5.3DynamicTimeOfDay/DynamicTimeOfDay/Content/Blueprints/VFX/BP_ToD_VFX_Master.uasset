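; Master VFX actor that shows a configurable Niagara effect at night and hides it by day when linked to BP_TimeOfDay.
; The construction script assigns the system, applies an emissive-scaled color and previews the on/off state from the current hour.
; At BeginPlay, after a short delay, it finds the TimeOfDay actor, binds to its day and night events, and sets the initial state by toggling visibility and activation.
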(event `self.ReceiveBeginPlay`
  (`KismetSystemLibrary.Delay` 0.04)
  ;[1 1 1] TimeOfDay Actor Grab
  (if (`self.UseWithTimeOfDay`)
    (bind _returnvalue (`GameplayStatics.GetActorOfClass` "/DynamicTimeOfDay/Blueprints/TimeOfDay/BP_TimeOfDay.BP_TimeOfDay_C"))
    (`/Engine/EditorBlueprintResources/StandardMacros.IsValid` _returnvalue
      (:`Is Valid`
        (set `self.TimeOfDayActor` _returnvalue))
      (:`Is Not Valid`
        _)))
  (`self.BindEvents`)
  (`self.StartupOnOff`))

(event `StartupOnOff`
  (bind _timeofdayactor (`self.TimeOfDayActor`))
  (bind (_daystarthour _nightstarthour) (break `DayNightEvents` (`TimeOfDay.DayNightEvents` _timeofdayactor)))
  ;[1 1 1] Startup On Off
  (if (`self.UseWithTimeOfDay`)
    (`/Engine/EditorBlueprintResources/StandardMacros.IsValid` _timeofdayactor
      (:`Is Valid`
        (if (`KismetMathLibrary.InRange_FloatFloat` (`.Hour` (break `BaseSetup` (`TimeOfDay.BaseSetup` _timeofdayactor))) _daystarthour _nightstarthour)
          (`self.SetOFF`)
          (else
            (`self.SetOn`)))))))

(event `SetON`
  (bind _niagaraparticle (`self.NiagaraParticle`))
  (`/Engine/EditorBlueprintResources/StandardMacros.IsValid` (`self.NiagaraSystem`)
    (:`Is Valid`
      (`SceneComponent.SetVisibility` _niagaraparticle true false)
      (`ActorComponent.Activate` _niagaraparticle true))))

(event `BindEvents`
  (bind _timeofdayactor (`self.TimeOfDayActor`))
  ;[1 1 1] Bind Events
  (if (`self.UseWithTimeOfDay`)
    (`/Engine/EditorBlueprintResources/StandardMacros.IsValid` _timeofdayactor
      (:`Is Valid`
        (add `/DynamicTimeOfDay/Blueprints/TimeOfDay/BP_TimeOfDay.SetDay` _timeofdayactor (`|CreateDelegate` :!event `SetOn`))
        (add `/DynamicTimeOfDay/Blueprints/TimeOfDay/BP_TimeOfDay.SetNight` _timeofdayactor (`|CreateDelegate` :!event `SetOFF`))))))

(event `SetOFF`
  (bind _niagaraparticle (`self.NiagaraParticle`))
  (`/Engine/EditorBlueprintResources/StandardMacros.IsValid` (`self.NiagaraSystem`)
    (:`Is Valid`
      (`SceneComponent.SetVisibility` _niagaraparticle false false)
      (`ActorComponent.Deactivate` _niagaraparticle))))

(fn `UserConstructionScript`
  (locals (NewLocalVar_0 :type "Float (single-precision)" :default 0.0))
  (bind _emissivescale (`self.EmissiveScale`))
  (bind (_r _g _b _a) (`KismetMathLibrary.BreakColor` (`self.Color`)))
  (`/Engine/EditorBlueprintResources/StandardMacros.IsValid` (`self.NiagaraSystem`)
    (:`Is Valid`
      (`NiagaraComponent.SetAsset` (`self.NiagaraParticle`) (`self.NiagaraSystem`) true)
      (`|ExecutionSequence`
        (:`then_0`
          (`FXSystemComponent.SetColorParameter` (`self.NiagaraParticle`) "Color" (make `LinearColor` (* _r _emissivescale) (* _g _emissivescale) (* _b _emissivescale) _a)))
        (:`then_1`
          (if (`self.UseWithTimeOfDay`)
            (bind _returnvalue (`GameplayStatics.GetActorOfClass` "/DynamicTimeOfDay/Blueprints/TimeOfDay/BP_TimeOfDay.BP_TimeOfDay_C"))
            (bind (_daystarthour _nightstarthour) (break `DayNightEvents` (`TimeOfDay.DayNightEvents` _returnvalue)))
            (if (`KismetMathLibrary.InRange_FloatFloat` (`.Hour` (break `BaseSetup` (`TimeOfDay.BaseSetup` _returnvalue))) _daystarthour _nightstarthour)
              (`self.SetOFF`)
              (else
                (`self.SetOn`)))
            (else
              (`self.SetOn`))))))))